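; Player character Blueprint for a 2D side-scrolling Megaman, with run, jump, ground and air dash, and three projectile attacks.
; Input handlers launch the character and temporarily suspend gravity and falling friction for dashes and heavy shots.
; A shared FireProjectile macro spawns shots and applies recoil, using DoN counters that, like jumps and air dashes, reset on landing.
; Tick updates air state and calls UpdateAnimation, which maps movement flags to flipbooks.
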(event `self.ReceiveBeginPlay`
  (bind _charactermovement (`self.CharacterMovement`))
  ;[1 1 1] BeginPlay
  (set `self.DefaultGravityScale` (`CharacterMovementComponent.GravityScale` _charactermovement))
  (set `self.DefaultMaxWalkSpeed` (`CharacterMovementComponent.MaxWalkSpeed` _charactermovement))
  (set `self.DefaultFallingLateralFriction` (`CharacterMovementComponent.FallingLateralFriction` _charactermovement))
  (set `self.DefaultGroundFriction` (`CharacterMovementComponent.GroundFriction` _charactermovement)))

(event `self.ReceiveTick`
  (params (DeltaSeconds :type "Float (single-precision)"))
  (bind (_returnvalue_x _returnvalue_y _returnvalue_z) (`KismetMathLibrary.BreakVector` (`self.GetVelocity`)))
  ;[1 1 1] Rotate Camera & Controls
  (if (`NavMovementComponent.IsMovingOnGround` (`self.CharacterMovement`))
    (set `self.isInAir` false)
    (`self.ResetAllAirCounters`)
    (else
      (set `self.isInAir` true)))
  (if (<= _returnvalue_z 0.0)
    (set `self.isFalling` true)
    (else
      (set `self.isFalling` false)))
  (`self.UpdateAnimation`))

(event `ResetAllAirCounters`
  ;[1 1 1] Rotate Camera & Controls
  (`self.ResetJumpCount`)
  (`self.ResetAirRecoil`)
  (`self.ResetAirDash`)
  (`self.ResetMediumAirRecoil`))

(event `InputAxis|MoveRight`
  (params (AxisValue :type "Float (single-precision)"))
  ;[1 1 1] Directional Input
  (if (not (or (`self.isDashing`) (`self.isAltFiring`) (and (`self.isFiring`) (`self.isInAir`))))
    (if (> AxisValue 0.0)
      (set `self.isMovingRight` true)
      (`self.AddMovementInput` (1.0 0.0 0.0) AxisValue :!label _label)
      (`/Engine/EditorBlueprintResources/StandardMacros.CompareFloat` AxisValue
        (:`>`
          (`Controller.SetControlRotation` (`self.GetController`) (`KismetMathLibrary.MakeRotator` 0.0 0.0 0.0)))
        (:`<`
          (`Controller.SetControlRotation` (`self.GetController`) (`KismetMathLibrary.MakeRotator` 0.0 0.0 180.0))))
      (elif (< AxisValue 0.0)
        (set `self.isMovingRight` false)
        (goto _label)))))

(event `InputAxis|Jump`
  (params (AxisValue :type "Float (single-precision)"))
  ;[1 1 1] Jump & Slide
  (if (and (>= AxisValue 0.4) (`self.isFalling`) (`KismetMathLibrary.BooleanNOR` (`self.isAltFiring`) (`self.isDashing`)))
    (set `self.isSliding` false)
    (`/Engine/EditorBlueprintResources/StandardMacros.Do N` (`self.MaxJumpCount`) :!label _label_2
      (:`Exit`
        (`self.LaunchCharacter` (`KismetMathLibrary.MakeVector` 0.0 0.0 (`CharacterMovementComponent.JumpZVelocity` (`self.CharacterMovement`))) false true)
        (`GameplayStatics.PlaySound2D` "/Game/Sounds/Jump.Jump")
        (`self.ResetAirRecoil`)))
    (elif (<= AxisValue -0.3)
      (set `self.isSliding` true)
      (else
        (set `self.isSliding` false)))))

(event `ResetJumpCount`
  ;[1 1 1] Jump & Slide
  (goto _label_2 :!via `Reset`))

(event `InputAction|AltFire`
  (params (Key :type "Key Structure" :default "AnyKey"))
  (bind _altfireprojectilerecoilduration (`self.AltFireProjectileRecoilDuration`))
  (bind _charactermovement (`self.CharacterMovement`))
  (bind _charactermovement_2 (`self.CharacterMovement`))
  (bind _altfireprojectilerecoil (`self.AltFireProjectileRecoil`))
  ;[1 1 1] AltFire
  (:`Pressed`
    (if (`self.canAltFire`)
      (if (not (and (`self.isDashing`) (`self.isUltimating`) (`self.isAltFiring`)))
        (set `CharacterMovementComponent.GravityScale` 0.0 _charactermovement)
        (set `CharacterMovementComponent.FallingLateralFriction` 0.0 _charactermovement)
        (set `self.canAltFire` false)
        (set `self.isAltFiring` true)
        (`self.FireProjectile` (`|GetArrayItem` (`self.ProjectileType`) 1) (`self.AltFireProjectileRecoil`) (`self.MediumProjectileSound`) :!label _label_3
          (:`ShootsFired`
            (if (not (`self.isInAir`))
              (if (`self.isMovingRight`)
                (`self.LaunchCharacter` (`KismetMathLibrary.MakeVector` (* _altfireprojectilerecoil -0.5)) true)
                (else
                  (`self.LaunchCharacter` (`KismetMathLibrary.MakeVector` (* _altfireprojectilerecoil 0.5)) true))))))))
    (`KismetSystemLibrary.Delay` _altfireprojectilerecoilduration)
    (set `CharacterMovementComponent.GravityScale` (`self.DefaultGravityScale`) _charactermovement_2)
    (set `CharacterMovementComponent.FallingLateralFriction` (`self.DefaultFallingLateralFriction`) _charactermovement_2)
    (`KismetSystemLibrary.Delay` (- (`self.AltFireCooldown`) _altfireprojectilerecoilduration))
    (set `self.canAltFire` true)
    (set `self.isAltFiring` false)))

(event `ResetMediumAirRecoil`
  ;[1 1 1] AltFire
  (goto _label_3 :!via `ResetAirRecoils`))

(event `InputTouch`
  (params (Location :type "Vector Structure") (FingerIndex :type "ETouchIndex Enum"))
  ;[1 1 1] Dash On Swipe
)

(event `InputAction|Fire`
  (params (Key :type "Key Structure" :default "AnyKey"))
  ;[1 1 1] Firing Small Projectiles
  (:`Pressed`
    (if (not (`self.isDashing`))
      (set `self.isFiring` true)
      (`self.FireProjectile` (`|GetArrayItem` (`self.ProjectileType`)) (`self.SmallProjectileRecoil`) (`self.SmallProjectileSound`) :!label _label_4
        (:`ShootsFired`
          (bind _returnvalue (`KismetSystemLibrary.K2_SetTimerDelegate` (delegate `Fire`) (/ 1.0 (`self.BulletsPerSecond`)) true))
          (set `self.FireTimer` _returnvalue)))))
  (:`Released`
    (set `self.isFiring` false)
    (`KismetSystemLibrary.K2_ClearAndInvalidateTimerHandle` (`self.FireTimer`))))

(event `ResetAirRecoil`
  ;[1 1 1] Firing Small Projectiles
  (`|ExecutionSequence`
    (:`then_0`
      (goto _label_4 :!via `ResetAirRecoils`))
    (:`then_1`
      (goto _label_5 :!via `ResetAirRecoils`))))

(event `Fire`
  ;[1 1 1] Firing Small Projectiles
  (`self.FireProjectile` (`|GetArrayItem` (`self.ProjectileType`)) (`self.SmallProjectileRecoil`) (`self.SmallProjectileSound`) :!label _label_5))

(event `InputAction|Dash`
  (params (Key :type "Key Structure" :default "AnyKey"))
  (bind _charactermovement (`self.CharacterMovement`))
  (bind _charactermovement_2 (`self.CharacterMovement`))
  (bind _charactermovement_3 (`self.CharacterMovement`))
  (bind _dashlaunch (`self.DashLaunch`))
  (bind _charactermovement_4 (`self.CharacterMovement`))
  (bind _dashlaunch_2 (`self.DashLaunch`))
  (bind _charactermovement_5 (`self.CharacterMovement`))
  (bind _charactermovement_6 (`self.CharacterMovement`))
  (:`Pressed`
    (if (`self.canDash`)
      (if (`NavMovementComponent.IsMovingOnGround` (`self.CharacterMovement`))
        ;[1 1 1] Ground Dash
        (set `self.canDash` false)
        (set `self.isDashing` true)
        (set `CharacterMovementComponent.GravityScale` 0.0 _charactermovement_4)
        (set `CharacterMovementComponent.FallingLateralFriction` 0.0 _charactermovement_4)
        (if (`self.isMovingRight`)
          (`self.LaunchCharacter` (`KismetMathLibrary.MakeVector` _dashlaunch_2) true true)
          (else
            (`self.LaunchCharacter` (`KismetMathLibrary.MakeVector` (* _dashlaunch_2 -1.0)) true true)))
        (`GameplayStatics.PlaySound2D` "/Game/Sounds/GroundDash.GroundDash")
        (`KismetSystemLibrary.Delay` (`self.DashMaxDuration`))
        (set `CharacterMovementComponent.GravityScale` (`self.DefaultGravityScale`) _charactermovement_5)
        (set `CharacterMovementComponent.FallingLateralFriction` (`self.DefaultFallingLateralFriction`) _charactermovement_5)
        (set `self.isDashing` false)
        (set `self.canDash` true)
        (else
          ;[1 1 1] Air Dash
          (`/Engine/EditorBlueprintResources/StandardMacros.Do N` (`self.NbAirDashes`) :!label _label_6
            (:`Exit`
              (set `self.canDash` false)
              (set `self.isDashing` true)
              (set `self.isAirDashing` true)
              (`self.ResetAirRecoil`)
              (set `CharacterMovementComponent.GravityScale` 0.0 _charactermovement)
              (set `CharacterMovementComponent.FallingLateralFriction` 0.0 _charactermovement)
              (set `MovementComponent.Velocity` (0.0 0.0 0.0) _charactermovement)
              (`KismetSystemLibrary.Delay` (`self.AirDashDelay`))
              (if (`self.isMovingRight`)
                (`self.LaunchCharacter` (`KismetMathLibrary.MakeVector` _dashlaunch) false true)
                (else
                  (`self.LaunchCharacter` (`KismetMathLibrary.MakeVector` (* _dashlaunch -1.0)) false true)))
              (`GameplayStatics.PlaySound2D` "/Game/Sounds/Flying.Flying")
              (`KismetSystemLibrary.Delay` (`self.DashMaxDuration`))
              (set `CharacterMovementComponent.GravityScale` (`self.DefaultGravityScale`) _charactermovement_2)
              (set `CharacterMovementComponent.FallingLateralFriction` (`self.DefaultFallingLateralFriction`) _charactermovement_2)
              (set `self.isDashing` false)
              (set `self.isAirDashing` false)
              (`KismetSystemLibrary.Delay` 0.2)
              (set `self.canDash` true)))))))
  (:`Released`
    ;[1 1 1] Dash Input Release
    (if (`self.isAirDashing`)
      (`KismetSystemLibrary.Delay` (`self.AirDashDelay`))
      (set `self.isDashing` false)
      (set `self.isAirDashing` false)
      (set `CharacterMovementComponent.GravityScale` (`self.DefaultGravityScale`) _charactermovement_3)
      (set `CharacterMovementComponent.FallingLateralFriction` (`self.DefaultFallingLateralFriction`) _charactermovement_3)
      (else
        (set `self.isDashing` false)
        (set `CharacterMovementComponent.GravityScale` (`self.DefaultGravityScale`) _charactermovement_6)
        (set `CharacterMovementComponent.FallingLateralFriction` (`self.DefaultFallingLateralFriction`) _charactermovement_6)))))

(event `InputAction|Ultimate`
  (params (Key :type "Key Structure" :default "AnyKey"))
  (bind _charactermovement (`self.CharacterMovement`))
  (bind _ultimateprojectilerecoil (`self.UltimateProjectileRecoil`))
  (bind _ultimateprojectilerecoilduration (`self.UltimateProjectileRecoilDuration`))
  (bind _charactermovement_2 (`self.CharacterMovement`))
  ;[1 1 1] Ultimate
  (:`Pressed`
    (if (and (`self.canUlt`) (not (`self.isDashing`)) (not (`self.isAltFiring`)))
      (set `CharacterMovementComponent.GravityScale` 0.0 _charactermovement_2)
      (set `CharacterMovementComponent.FallingLateralFriction` 0.0 _charactermovement_2)
      (set `self.canUlt` false)
      (set `self.isUltimating` true)
      (`self.FireProjectile` (`|GetArrayItem` (`self.ProjectileType`) 2) (`self.UltimateProjectileRecoil`) (`self.LargeProjectileSound`) :!label _label_7
        (:`ShootsFired`
          (if (not (`self.isInAir`))
            (if (`self.isMovingRight`)
              (`self.LaunchCharacter` (`KismetMathLibrary.MakeVector` (* _ultimateprojectilerecoil -0.5)) true)
              (else
                (`self.LaunchCharacter` (`KismetMathLibrary.MakeVector` (* _ultimateprojectilerecoil 0.5)) true))))
          (`KismetSystemLibrary.Delay` _ultimateprojectilerecoilduration))))
    (set `self.isAltFiring` false)
    (set `CharacterMovementComponent.GravityScale` (`self.DefaultGravityScale`) _charactermovement)
    (set `CharacterMovementComponent.FallingLateralFriction` (`self.DefaultFallingLateralFriction`) _charactermovement)
    (`KismetSystemLibrary.Delay` (- (`self.UltimateCooldown`) _ultimateprojectilerecoilduration))
    (set `self.canAltFire` true)))

(event `CustomEvent`
  ;[1 1 1] Ultimate
  (goto _label_7 :!via `ResetAirRecoils`))

(event `ResetAirDash`
  ;[1 1 1] Air Dash
  (goto _label_6 :!via `Reset`))

(fn `UpdateAnimation`
  (bind (_megaman_flipbooks_idle _megaman_flipbooks_run _megaman_flipbooks_jump _megaman_flipbooks_inair _megaman_flipbooks_fire _megaman_flipbooks_fireair _megaman_flipbooks_fireinair _megaman_flipbooks_firerun _megaman_flipbooks_dash _megaman_flipbooks_aerial _megaman_flipbooks_slide) (break `/Game/Sprites/Megaman/PaperFlipbooks/Megaman_Flipbooks` (`self.Megaman_Flipbooks`)))
  (if (`self.isDashing`)
    (if (`self.isAirDashing`)
      (set `self.Megaman_PlayerState` "NewEnumerator9")
      (elif (not (`self.isSliding`))
        (set `self.Megaman_PlayerState` "NewEnumerator8")
        (else
          (set `self.Megaman_PlayerState` "NewEnumerator10"))))
    (`PaperFlipbookComponent.SetLooping` (`self.Sprite`) false :!label _label)
    (elif (`self.isAltFiring`)
      (set `self.Megaman_PlayerState` "NewEnumerator4")
      (goto _label)
      (else
        (if (== (`KismetMathLibrary.VSize` (`self.GetVelocity`)) 0.0)
          (if (`self.isFiring`)
            (set `self.Megaman_PlayerState` "NewEnumerator4")
            (else
              (set `self.Megaman_PlayerState` "NewEnumerator0")))
          (elif (not (`self.isInAir`))
            (if (`self.isFiring`)
              (set `self.Megaman_PlayerState` "NewEnumerator7")
              (else
                (set `self.Megaman_PlayerState` "NewEnumerator1")))
            (elif (not (`self.isFalling`))
              (if (`self.isFiring`)
                (set `self.Megaman_PlayerState` "NewEnumerator5")
                (goto _label)
                (else
                  (set `self.Megaman_PlayerState` "NewEnumerator2")
                  (goto _label)))
              (elif (`self.isFiring`)
                (set `self.Megaman_PlayerState` "NewEnumerator6")
                (else
                  (set `self.Megaman_PlayerState` "NewEnumerator3"))))))
        (`PaperFlipbookComponent.SetLooping` (`self.Sprite`) true)
        (`PaperFlipbookComponent.Play` (`self.Sprite`)))))
  (`PaperFlipbookComponent.SetFlipbook` (`self.Sprite`) (select `/Game/Sprites/Megaman/PaperFlipbooks/Megaman_PlayerState` (`self.Megaman_PlayerState`) :`NewEnumerator0` _megaman_flipbooks_idle :`NewEnumerator1` _megaman_flipbooks_run :`NewEnumerator2` _megaman_flipbooks_jump :`NewEnumerator3` _megaman_flipbooks_inair :`NewEnumerator4` _megaman_flipbooks_fire :`NewEnumerator5` _megaman_flipbooks_fireair :`NewEnumerator6` _megaman_flipbooks_fireinair :`NewEnumerator7` _megaman_flipbooks_firerun :`NewEnumerator8` _megaman_flipbooks_dash :`NewEnumerator9` _megaman_flipbooks_aerial :`NewEnumerator10` _megaman_flipbooks_slide)))

(fn `UserConstructionScript`)